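; Clue actor that randomizes its appearance on BeginPlay and is meant to raise enemy suspicion.
; It sets the Cube mesh from a random MeshArray entry, using an index range that skips element zero.
; A second, independent random roll picks a SuspicionLevelArray value to add to Enemy_Controller's Suspicion, so mesh and amount are unlinked.
; The Enemy_Controller cast shows no object input, so that addition depends on a cast with nothing to resolve.
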(event EventBeginPlay
  (bind _returnvalue (Math|Random|RandomIntegerinRange 1 4))
  (Components|StaticMesh|SetStaticMesh (Variables|Default|GetCube) (Utilities|Array|Get(acopy) (Variables|Default|GetMeshArray) _returnvalue))
  (bind _asenemy_controller (Utilities|Casting|CastToEnemy_Controller))
  (Variables|/Game/Enemy/Enemy_Controller.Enemy_Controller_C|SetSuspicion _asenemy_controller (+ (Utilities|Array|Get(acopy) (Variables|Default|GetSuspicionLevelArray) _returnvalue) (Variables|/Game/Enemy/Enemy_Controller.Enemy_Controller_C|GetSuspicion _asenemy_controller))))

(fn ConstructionScript)